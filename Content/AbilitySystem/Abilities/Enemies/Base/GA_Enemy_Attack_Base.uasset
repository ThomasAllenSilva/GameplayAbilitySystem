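; Base enemy attack gameplay ability that plays a random attack montage and damages player characters caught in the hit area.
; On activation it sets the owner's motion warp target to the target actor's location, then plays the montage.
; The Common.Event.Attack gameplay event triggers a sphere overlap that applies damage to each player found.
; GetAttackOverlapLocation returns a zero vector here, and the ability ends when the montage completes, is interrupted or is cancelled.
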(event Ability|EventActivateAbility
  (bind _ownerauracharacter (Variables|Default|GetOwnerAuraCharacter))
  ;[1 1 1] Update Warp Target To Where We Want To Rotate
  (Class|AuraCharacterBase|UpdateWarpTargetfromLocation _ownerauracharacter (Class|AuraCharacterBase|GetTargetActorLocation _ownerauracharacter))
  ;[1 1 1] Play The Attack Montage
  (|PlayMontageandWaitProxy "None" (CallFunction|GetAttackMontage) 1.0 "None" true 1.0 0.0 false
    (:then
      (Ability|Tasks|WaitGameplayEvent "(TagName=\"Common.Event.Attack\")" 0
        (:EventReceived
          ;[1 1 1] Apply Damage To Each Target Inside The Attack Area
          (bind _outactors (Collision|SphereOverlapActors (CallFunction|GetAttackOverlapLocation) 1e+02 (Variables|Default|GetOverlap%20Object%20Types) "/Script/Aura.AuraPlayerCharacter" (Utilities|Array|MakeArray (Ability|GetAvatarActorfromActorInfo))))
          (for _array_element _outactors
            (Class|AuraDamageGameplayAbility|ApplyDamage _array_element)))))
    (:OnCompleted
      (Ability|EndAbility :!label _label))
    (:OnInterrupted
      (goto _label))
    (:OnCancelled
      (goto _label))))

(fn GetAttackOverlapLocation
  (return "0, 0, 0"))

(fn GetAttackMontage
  (return (Utilities|Array|Get(acopy) (Variables|Default|GetAttack%20Montages) (Math|Random|RandomInteger (Utilities|Array|Length (Variables|Default|GetAttack%20Montages))))))