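; Base gameplay ability for ranged enemy attacks that fires a projectile at the enemy's current target.
; On activation it sets the motion warp target to the target's location and plays the attack montage.
; An attack gameplay event during the montage spawns the projectile from the weapon socket toward the target's position at that moment.
; The ability ends when the montage completes, is interrupted or is cancelled.
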(event Ability|EventActivateAbility
  (bind _returnvalue (Class|AuraGameplayAbility|GetAuraCharacterfromActorInfo))
  ;[1 1 1] Update Warp Target To Where We Want To Rotate
  (Class|AuraCharacterBase|UpdateWarpTargetfromLocation _returnvalue (Class|AuraEnemyCharacter|GetTargetActorLocation _returnvalue))
  ;[1 1 1] Play The Attack Montage
  (|PlayMontageandWaitProxy "None" (Variables|Default|GetAttack%20Montage) 1.0 "None" false 1.0 0.0 false
    (:then
      (Ability|Tasks|WaitGameplayEvent "(TagName=\"Common.Event.Attack\")" 0
        (:EventReceived
          ;[1 1 1] Spawn The Projectile Towards The Target Location
          (Class|AuraProjectileSpell|SpawnProjectile (Class|AuraEnemyCharacter|GetTargetActorLocation (Class|AuraGameplayAbility|GetAuraCharacterfromActorInfo))))))
    (:OnCompleted
      (Ability|EndAbility :!label _label))
    (:OnInterrupted
      (goto _label))
    (:OnCancelled
      (goto _label))))

(fn GetProjectileSpawnLocation
  (return (Class|AuraCharacterBase|GetWeaponSocketLocation (Class|AuraGameplayAbility|GetAuraCharacterfromActorInfo))))