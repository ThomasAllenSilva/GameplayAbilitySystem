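; Gameplay ability for the Ghoul enemy's attack that supplies the location of the attack overlap.
; It overrides or implements only GetAttackOverlapLocation, matching the current montage against the first entry in AttackMontages to pick the hand.
; That first montage selects the LeftHand socket and any other selects RightHand, whose location on the owning component is returned.
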(fn GetAttackOverlapLocation
  (Utilities|FlowControl|Sequence
    (:then_0
      ;[1 1 1] Check Which Hand We're Using To Attack And Set The Hand Socket
      (if (== (Animation|GetCurrentMontage :!class /Script/GameplayAbilities.GameplayAbility) (Utilities|Array|Get(acopy) (Variables|Default|GetAttack%20Montages)))
        (LocalVariables|SetSocket%20Name "LeftHand")
        (else
          (LocalVariables|SetSocket%20Name "RightHand"))))
    (:then_1
      ;[1 1 1] Return The Corresponding Hand Socket
      (return (Transformation|GetSocketLocation (Class|GameplayAbility|GetOwningComponentfromActorInfo) (LocalVariables|GetSocket%20Name))))))