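; Shaman enemy gameplay ability that summons random minions at computed spawn locations during a summon montage.
; Ground-summon Niagara effects mark each location, then a Common.Event.Attack gameplay event starts a staggered Delay loop that spawns one minion per location.
; Each spawn increments the owner's minion count, and its OnDestroyed binding calls the decrement.
; The ability ends when the montage completes, blends out or is cancelled; SpawnDemons only sets timers, spawning nothing itself.
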(event Custom|On%20Minion%20Died
  (params (DestroyedActor :type Actor%20Object%20Reference))
  (Class|AuraElementalistEnemyCharacter|DecrementMinionsCount (Class|AuraSummonMinionsAbility|GetElementalistEnemyCharacterfromActorInfo) -1))

(event Ability|EventActivateAbility
  (Variables|Default|SetCurrent%20Spawn%20Locations (Class|AuraSummonMinionsAbility|GetSpawnLocations))
  (|PlayMontageandWaitProxy "None" "/Game/Assets/Enemies/Shaman/Animations/Shaman_Summon_Montage.Shaman_Summon_Montage" 1.0 "None" true 1.0 0.0 false
    (:then
      (CallFunction|DisplaySummonParticles)
      (Ability|Tasks|WaitGameplayEvent "(TagName=\"Common.Event.Attack\")" 0 true
        (:EventReceived
          (CallFunction|SpawnDemons)
          (Variables|Default|SetSpawn%20Index 0)
          (if (< (Variables|Default|GetSpawn%20Index) (Utilities|Array|Length (Variables|Default|GetCurrent%20Spawn%20Locations))) :!label _label
            (bind _returnvalue (Class|AuraSummonMinionsAbility|SpawnRandomMinion (Math|Transform|MakeTransform (Utilities|Array|Get(acopy) (Variables|Default|GetCurrent%20Spawn%20Locations) (Variables|Default|GetSpawn%20Index)) "0, 0, 0" "1.000000,1.000000,1.000000")))
            (Math|Integer|IncrementInt (Variables|Default|GetSpawn%20Index)
              (:%20%20
                (Game|AssignOnDestroyed _returnvalue (delegate Custom|On%20Minion%20Died))
                (Class|AuraElementalistEnemyCharacter|IncrementMinionsCount (Class|AuraSummonMinionsAbility|GetElementalistEnemyCharacterfromActorInfo) 1)
                (Utilities|FlowControl|Delay 0.2)
                (goto _label)))))))
    (:OnCompleted
      (Ability|EndAbility :!label _label_2))
    (:OnBlendOut
      (goto _label_2))
    (:OnCancelled
      (goto _label_2))))

(fn DisplaySummonParticles
  (for _array_element (Variables|Default|GetCurrent%20Spawn%20Locations)
    (Niagara|SpawnSystematLocation "/Game/Assets/Effects/Combat/NS_GroundSummon.NS_GroundSummon" _array_element)))

(fn SpawnDemons
  (for _array_element (Variables|Default|GetCurrent%20Spawn%20Locations)
    (Utilities|Time|SetTimerbyEvent (EventDispatchers|CreateEvent :!event GAShamanSummonMinionAutoGenFunc) 0.0)))

(fn GAShamanSummonMinionAutoGenFunc
  (Development|PrintString "Spawn!"))