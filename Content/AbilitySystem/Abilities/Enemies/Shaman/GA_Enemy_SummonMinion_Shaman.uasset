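; Enemy Shaman gameplay ability that summons random minions during an attack montage.
; When the montage's attack gameplay event arrives, it spawns a random minion at each computed spawn location, facing the avatar's rotation.
; Each spawn increments the minion count on the Elementalist enemy character, and a bound OnDestroyed handler calls DecrementMinionsCount when that minion is destroyed.
; The ability ends when the montage completes, is interrupted or is cancelled.
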(event Custom|On%20Minion%20Died
  (params (DestroyedActor :type Actor%20Object%20Reference))
  (Class|AuraElementalistEnemyCharacter|DecrementMinionsCount (Class|AuraSummonMinionsAbility|GetElementalistEnemyCharacterfromActorInfo) -1))

(event Ability|EventActivateAbility
  (|PlayMontageandWaitProxy "None" "/Game/Assets/Enemies/Shaman/Animations/Shaman_Summon_Montage.Shaman_Summon_Montage" 1.0 "None" true 1.0 0.0 false
    (:then
      (Ability|Tasks|WaitGameplayEvent "(TagName=\"Common.Event.Attack\")" 0
        (:EventReceived
          (for _array_element (Class|AuraSummonMinionsAbility|GetSpawnLocations)
            (bind _returnvalue (Class|AuraSummonMinionsAbility|SpawnRandomMinion (Math|Transform|MakeTransform _array_element (Transformation|GetActorRotation (Ability|GetAvatarActorfromActorInfo)) "1.000000,1.000000,1.000000")))
            (Game|AssignOnDestroyed _returnvalue (delegate Custom|On%20Minion%20Died))
            (Class|AuraElementalistEnemyCharacter|IncrementMinionsCount (Class|AuraSummonMinionsAbility|GetElementalistEnemyCharacterfromActorInfo) 1)))))
    (:OnCompleted
      (Ability|EndAbility :!label _label))
    (:OnInterrupted
      (goto _label))
    (:OnCancelled
      (goto _label))))