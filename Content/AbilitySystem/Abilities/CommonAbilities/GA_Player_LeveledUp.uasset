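; Player level-up gameplay ability, activated by a gameplay event, that gives feedback and grants upgrade points, then ends.
; It spawns an attached Niagara effect, plays a 2D sound, and shows a level message widget, removing any previous one first.
; It looks up attribute and ability point awards for the current level in UpgradeInfo and applies them to the owner through GE_UpgradeAwards using SetByCaller magnitudes.
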(event Ability|EventActivateAbilityFromEvent
  (params (EventData :type Gameplay%20Event%20Data%20Structure%20%28by%20ref%29))
  (CallFunction|SpawnLevelUpNiagaraSystem)
  (CallFunction|PlayLevelUpSound2D)
  (CallFunction|DisplayLevelUpWidget)
  (CallFunction|Award)
  (Ability|EndAbility))

(fn SpawnLevelUpNiagaraSystem
  (bind _ownerauracharacter (Variables|Default|GetOwnerAuraCharacter))
  (Niagara|SpawnSystemAttached "/Game/Assets/Effects/LevelUp/NS_LevelUp.NS_LevelUp" (Variables|/Script/Engine.Actor|GetRootComponent _ownerauracharacter) "None" (Transformation|GetActorLocation _ownerauracharacter) (Camera|GetCameraRotation (Variables|/Script/Engine.PlayerController|GetPlayerCameraManager (Class|CommonAbilityFunctionLibrary|GetLocalPlayerController))) "KeepWorldPosition" true true "AutoRelease"))

(fn PlayLevelUpSound2D
  (Audio|PlaySound2D "/Game/Assets/Sounds/LevelUp/sfx_LeveledUp.sfx_LeveledUp" 1.0 1.0 0.0 0 0))

(fn DisplayLevelUpWidget
  (CallFunction|TryClearCurrentLeveledUpWidget)
  (bind _returnvalue (UserInterface|CreateWidget "/Game/Widgets/Player/LeveledUp/WBP_Player_LeveledUpMessage.WBP_Player_LeveledUpMessage_C"))
  (Variables|Default|SetCurrent%20Leveled%20Up%20Widget _returnvalue)
  (Default|SetLevelText _returnvalue (.ReturnValue (Ability|Attribute|GetFloatAttribute (Variables|Default|GetOwnerAuraCharacter) "(AttributeName=\"Level\",Attribute=/Script/Aura.AuraExperienceAttributeSet:Level,AttributeOwner=\"/Script/CoreUObject.Class'/Script/Aura.AuraExperienceAttributeSet'\")")))
  (UserInterface|Viewport|AddtoViewport (Variables|Default|GetCurrent%20Leveled%20Up%20Widget) 0))

(fn TryClearCurrentLeveledUpWidget
  (bind _current_leveled_up_widget (Variables|Default|GetCurrent%20Leveled%20Up%20Widget)
    (:then
      (Widget|RemovefromParent _current_leveled_up_widget))
    (:else)))

(fn Award
  (bind _returnvalue (Class|AuraExperienceInterface|GetCurrentLevel(Message) (Ability|GetOwningActorfromActorInfo)))
  (LocalVariables|SetAttribute%20Points%20Award (.attributepointaward (Class|DataAssetLevelUpInfo|GetInformationforLevel (Variables|Default|GetUpgrade%20Info) _returnvalue)))
  (LocalVariables|SetAbility%20Points%20Award (.abilitypointaward (Class|DataAssetLevelUpInfo|GetInformationforLevel (Variables|Default|GetUpgrade%20Info) _returnvalue)))
  (bind _returnvalue_2 (Ability|GameplayEffect|AssignTagSetbyCallerMagnitude (Ability|MakeOutgoingGameplayEffectSpec "/Game/AbilitySystem/Player/Data/GE_UpgradeAwards.GE_UpgradeAwards_C") "(TagName=\"Attributes.UpgradePoints.AttributePoint\")" (LocalVariables|GetAttribute%20Points%20Award)))
  (bind _returnvalue_3 (Ability|GameplayEffect|AssignTagSetbyCallerMagnitude _returnvalue_2 "(TagName=\"Attributes.UpgradePoints.AbilityPoint\")" (LocalVariables|GetAbility%20Points%20Award)))
  (Ability|ApplyGameplayEffectSpecToOwner _returnvalue_3))