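; Player gameplay ability that casts a firebolt toward the world location under the cursor.
; On activation it commits, captures the cursor location, sets Aura's warp target to face it and plays the cast montage.
; The montage's FireBolt gameplay event spawns the projectile toward that captured point, and montage completion, interruption or cancellation ends the ability.
; Overrides supply the weapon socket as spawn location and draw it as a debug sphere.
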(event Ability|EventActivateAbility
  (Ability|CommitAbility)
  (bind _returnvalue (Class|AuraFunctionLibrary|GetCursorWorldLocation))
  ;[1 1 1] Update Warp Target To Where We Want To Rotate
  (Class|AuraCharacterBase|UpdateWarpTargetfromLocation (Class|AuraGameplayAbility|GetAuraCharacterfromActorInfo) _returnvalue)
  ;[1 1 1] Play The Attack Montage
  (|PlayMontageandWaitProxy "None" "/Game/Assets/Characters/Aura/Animations/Abilities/Cast_FireBolt_Montage.Cast_FireBolt_Montage" 1.0 "None" true 1.0 0.0 false
    (:then
      (Ability|Tasks|WaitGameplayEvent "(TagName=\"Event.Montage.FireBolt\")" 0
        (:EventReceived
          ;[1 1 1] Spawn The Projectile Towards The Target Location
          (Class|AuraProjectileSpell|SpawnProjectile _returnvalue))))
    (:OnCompleted
      (Ability|EndAbility :!label _label))
    (:OnInterrupted
      (goto _label))
    (:OnCancelled
      (goto _label))))

(fn GetProjectileSpawnLocation
  (return (Class|AuraCharacterBase|GetWeaponSocketLocation (Class|AuraGameplayAbility|GetAuraCharacterfromActorInfo))))

(fn DisplayDebugInfo
  ;[1 1 1] Draw The Projectile Spawn Location
  (Rendering|Debug|DrawDebugSphere (Class|AuraCharacterBase|GetWeaponSocketLocation (Class|AuraGameplayAbility|GetAuraCharacterfromActorInfo)) 8.0 12 "(R=1.000000,G=1.000000,B=1.000000,A=1.000000)" 0.0))