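; Shared enemy base Blueprint that handles death with a ragdoll and a timed dissolve of body and weapon.
; On death it pauses animation, disables capsule collision, enables physics on the mesh and sets the actor's lifespan.
; It then swaps body and weapon to dynamic dissolve materials, using latent float lerps to drive their Dissolve parameter over that same lifespan.
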(event EventOnDied
  (CallFunction|ConfigureComponentstoDeath)
  (Actor|SetLifeSpan (Variables|Death|GetLifeSpanAfterDeath))
  (bind _returnvalue (Rendering|Material|CreateDynamicMaterialInstance (Variables|Death|GetCharacterDissolveMaterial) "None" "None" :!class /Script/Engine.KismetMaterialLibrary))
  (bind _output_get (Variables|Death|SetDynamicMeshMaterial _returnvalue))
  (Rendering|Material|SetMaterial (Variables|Character|GetMesh) 0 _output_get)
  (bind _lerpvalue (|LerpFloatWithinTime -0.55 0.55 (Variables|Death|GetLifeSpanAfterDeath))
    (:then
      (bind _returnvalue_2 (Rendering|Material|CreateDynamicMaterialInstance (Variables|Death|GetWeaponDissolveMaterial) "None" "None" :!class /Script/Engine.KismetMaterialLibrary))
      (bind _output_get_2 (Variables|Death|SetDynamicWeaponMaterial _returnvalue_2))
      (Rendering|Material|SetMaterial (Variables|Default|GetWeaponMesh) 0 _output_get_2)
      (bind _lerpvalue_2 (|LerpFloatWithinTime -0.55 0.55 (Variables|Death|GetLifeSpanAfterDeath))
        (:Tick
          _)
        (:Completed
          _))
      (Rendering|Material|SetScalarParameterValue (Variables|Death|GetDynamicWeaponMaterial) "Dissolve" _lerpvalue_2 :!class /Script/Engine.MaterialInstanceDynamic))
    (:Tick
      (Rendering|Material|SetScalarParameterValue (Variables|Death|GetDynamicMeshMaterial) "Dissolve" _lerpvalue :!class /Script/Engine.MaterialInstanceDynamic :!label _label))
    (:Completed
      (goto _label))))

(fn ConstructionScript)

(fn ConfigureComponentstoDeath
  (Variables|/Script/Engine.SkeletalMeshComponent|SetbPauseAnims (Variables|Character|GetMesh) true)
  (Collision|SetCollisionEnabled (Variables|Default|GetCapsuleComponent) "NoCollision")
  (Physics|SetSimulatePhysics (Variables|Character|GetMesh) true)
  (Collision|SetCollisionEnabled (Variables|Character|GetMesh) "QueryAndPhysics")
  (Physics|SetEnableGravity (Variables|Character|GetMesh) true)
  (Collision|SetCollisionResponsetoChannel (Variables|Character|GetMesh) "ECC_Pawn" "ECR_Block"))