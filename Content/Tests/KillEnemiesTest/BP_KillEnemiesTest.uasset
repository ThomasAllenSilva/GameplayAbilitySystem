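; Functional test that verifies enemies die when hit by lethal Gameplay Ability System damage.
; Every tick a kill trigger moves along world X, applying GE_Damage to overlapped actors that have an ability system component, with a huge set-by-caller Damage.Physical magnitude.
; After a fixed delay, the test fails if any actor in EnemiesToKill is still valid, otherwise it succeeds.
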(event OnActorBeginOverlap(KillTrigger)
  (params (OverlappedActor :type Actor%20Object%20Reference) (OtherActor :type Actor%20Object%20Reference))
  (bind _returnvalue (Ability|GetAbilitySystemComponent OtherActor))
  ;[1 1 1] Apply damage effect to each overlapped enemy with a magnitude sufficient to kill
  (Utilities|IsValid _returnvalue
    (:Is%20Valid
      (bind _returnvalue_2 (Ability|GameplayEffect|AssignTagSetbyCallerMagnitude (GameplayEffects|MakeOutgoingSpec :self _returnvalue :GameplayEffectClass "/Game/AbilitySystem/GameplayEffects/CommonEffects/GE_Damage.GE_Damage_C") "(TagName=\"Damage.Physical\")" 1e+16))
      (GameplayEffects|ApplyGameplayEffectSpecToSelf _returnvalue _returnvalue_2))))

(event EventStartTest
  ;[1 1 1] Wait a few seconds before checking if all the enemies died
  (Utilities|FlowControl|Delay 3.7)
  (for _array_element (Variables|Default|GetEnemies%20To%20Kill)
    (Utilities|IsValid _array_element
      (:Is%20Valid
        (Class|FunctionalTest|FinishTest "Failed" "Test Failed! Did not killed on time or enemy survived."))))
  (Class|FunctionalTest|FinishTest "Succeeded" "Test Succeeded! Killed all the enemies."))

(event EventTick
  (params (DeltaSeconds :type Float%20%28single-precision%29))
  ;[1 1 1] Move the kill trigger towards the enemies
  (Transformation|AddActorWorldOffset (Variables|Default|GetKill%20Trigger) "100.000000,0.000000,0.000000"))

(fn ConstructionScript)